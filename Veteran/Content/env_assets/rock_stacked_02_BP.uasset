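; Stacked rock environment Blueprint that acts as a one-way platform, solid only when the player is above it.
; Every Tick compares the static mesh's height with the player character mesh's, toggling collision on when the rock is lower and off otherwise.
; A component tagged JumpDown overlapping the Cube switches collision off for a brief delay to allow dropping through, though Tick keeps rewriting that same collision state during the delay.
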(event OnComponentBeginOverlap(Cube)
  (params (OverlappedComponent :type Primitive%20Component%20Object%20Reference) (OtherActor :type Actor%20Object%20Reference) (OtherComp :type Primitive%20Component%20Object%20Reference) (OtherBodyIndex :type Integer) (bFromSweep :type Boolean) (SweepResult :type Hit%20Result%20Structure%20%28by%20ref%29))
  (if (Components|ComponentHasTag OtherComp "JumpDown")
    (Collision|SetCollisionEnabled (Variables|Default|GetStaticMesh) "NoCollision")
    (Utilities|FlowControl|Delay 1.0)
    (Collision|SetCollisionEnabled (Variables|Default|GetStaticMesh) "QueryAndPhysics")))

(event EventTick
  (params (DeltaSeconds :type Float%20%28single-precision%29))
  (bind _staticmesh (Variables|Default|GetStaticMesh))
  (if (< (.Z (Math|Vector|BreakVector (Transformation|GetWorldLocation (Variables|Default|GetStaticMesh)))) (.Z (Math|Vector|BreakVector (Transformation|GetWorldLocation (Variables|/Script/Engine.Character|GetMesh (Game|GetPlayerCharacter 0))))))
    (Collision|SetCollisionEnabled _staticmesh "QueryAndPhysics")
    (else
      (Collision|SetCollisionEnabled _staticmesh "NoCollision"))))

(fn ConstructionScript)